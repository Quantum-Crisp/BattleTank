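; Player-controlled tank pawn Blueprint that wires components and input to movement, camera and firing logic.
; On BeginPlay it passes the barrel and turret references to the tank (for C++ use) and initialises the movement component with both tracks.
; Thumbstick input drives the movement component's intent functions, while trigger input throttles each track directly.
; Aim axes rotate an azimuth gimbal and spring arm separately to orbit the camera, and Fire launches a projectile.
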(event `self.ReceiveBeginPlay`
  ;[1 1 1] Find the barrel & turret component (For C++ use), and then find the tracks for the movement component
  (`self.SetBarrelReference` (`self.Barrel`))
  (`self.SetTurretReference` (`self.Turret`))
  (`TankMovementComponent.Initialise` (`self.MoveComponent`) (`self.LeftTrack`) (`self.RightTrack`)))

(event `InputAxis|MoveForward`
  (params (AxisValue :type "Float (single-precision)"))
  ;[1 1 1] Thumbstick Movement System
  (`TankMovementComponent.IntendMoveForward` (`self.MoveComponent`) AxisValue))

(event `InputAction|Fire`
  (params (Key :type "Key Structure"))
  ;[1 1 1] Fire a projectile
  (:`Pressed`
    (`self.Fire`)))

(event `InputAxis|TurnRight`
  (params (AxisValue :type "Float (single-precision)"))
  ;[1 1 1] Thumbstick Movement System
  (`TankMovementComponent.IntendTurnRight` (`self.MoveComponent`) AxisValue))

(event `InputAxis|AimElevation`
  (params (AxisValue :type "Float (single-precision)"))
  ;[1 1 1] Rotate the camera in the Y-axis
  (`SceneComponent.K2_AddLocalRotation` (`self.SpringArm`) (`KismetMathLibrary.MakeRotator` 0.0 AxisValue) false false))

(event `InputAxis|Left Track Throttle`
  (params (AxisValue :type "Float (single-precision)"))
  ;[1 1 1] Trigger Movement System
  (`TankTrack.SetThrottle` (`self.LeftTrack`) AxisValue))

(event `InputAxis|AimAzimuth`
  (params (AxisValue :type "Float (single-precision)"))
  ;[1 1 1] Rotate the camera in the X-axis
  (`SceneComponent.K2_AddLocalRotation` (`self.AzimuthGimbal`) (`KismetMathLibrary.MakeRotator` 0.0 0.0 AxisValue) false false))

(event `InputAxis|Right Track Throttle`
  (params (AxisValue :type "Float (single-precision)"))
  ;[1 1 1] Trigger Movement System
  (`TankTrack.SetThrottle` (`self.RightTrack`) AxisValue))

(fn `UserConstructionScript`)